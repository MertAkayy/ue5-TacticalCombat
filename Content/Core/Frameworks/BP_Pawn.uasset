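; BP_Pawn is a player camera pawn that moves, zooms and rotates through input.
; Axis inputs shift a desired location along the actor's forward and right vectors and adjust a desired spring arm length, with no clamping.
; Action inputs turn the desired rotation in 45-degree steps.
; Tick eases location, rotation and arm length toward these targets using interpolation helper functions, moving without sweep.
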(event EventTick
  (params (DeltaSeconds :type Float%20%28single-precision%29))
  (bind (_pawnspringarm _returnvalue) (CallFunction|CameraZoom DeltaSeconds))
  (Variables|/Script/Engine.SpringArmComponent|SetTargetArmLength _pawnspringarm _returnvalue)
  (Transformation|SetActorLocation (CallFunction|CameraMovement DeltaSeconds) false false)
  (Transformation|SetActorRotation (CallFunction|CameraRotation DeltaSeconds)))

(event EventBeginPlay
  (Variables|Default|SetDesiredLocation (Transformation|GetActorLocation))
  (Variables|Default|SetDesiredZoom (Variables|/Script/Engine.SpringArmComponent|GetTargetArmLength (Variables|Default|GetPawnSpringarm)))
  (Variables|Default|SetDesiredRotation (Transformation|GetActorRotation)))

(event Input|ActionEvents|InputActionCameraRotationRight
  (params (Key :type Key%20Structure :default "None"))
  ;[1 1 1] Rotate Camera 45 Degree Right
  (:Pressed
    (Variables|Default|SetDesiredRotation (Math|Rotator|CombineRotators (Variables|Default|GetDesiredRotation) "0.000000,-45.000000,0.000000"))))

(event Input|ActionEvents|InputActionCameraRotationLeft
  (params (Key :type Key%20Structure :default "None"))
  ;[1 1 1] Rotate Camera 45 Degree Left
  (:Pressed
    (Variables|Default|SetDesiredRotation (Math|Rotator|CombineRotators (Variables|Default|GetDesiredRotation) "0.000000,45.000000,0.000000"))))

(event Input|AxisEvents|InputAxisCameraZoom
  (params (AxisValue :type Float%20%28single-precision%29))
  ;[1 1 1] Camera Zoom in or out
  (Variables|Default|SetDesiredZoom (+ (* AxisValue 2e+02) (Variables|Default|GetDesiredZoom))))

(event Input|AxisEvents|InputAxisHorizontalMovement
  (params (AxisValue :type Float%20%28single-precision%29))
  ;[1 1 1] Move Pawn Forward or Backward
  (Variables|Default|SetDesiredLocation (+ (Variables|Default|GetDesiredLocation) (* (* AxisValue 1e+02) (Transformation|GetActorForwardVector)))))

(event Input|AxisEvents|InputAxisVerticalMovement
  (params (AxisValue :type Float%20%28single-precision%29))
  ;[1 1 1] Move Pawn to Right or Left
  (Variables|Default|SetDesiredLocation (+ (Variables|Default|GetDesiredLocation) (* (* AxisValue 1e+02) (Transformation|GetActorRightVector)))))

(fn ConstructionScript)

(fn CameraZoom
  (params (DeltaTime :type Float%20%28double-precision%29))
  (bind _pawnspringarm (Variables|Default|GetPawnSpringarm))
  (return _pawnspringarm (Math|Interpolation|FInterpTo (Variables|/Script/Engine.SpringArmComponent|GetTargetArmLength _pawnspringarm) (Variables|Default|GetDesiredZoom) DeltaTime 5.0)))

(fn CameraMovement
  (params (DeltaTime :type Float%20%28single-precision%29))
  (return (Math|Interpolation|VInterpTo (Transformation|GetActorLocation) (Variables|Default|GetDesiredLocation) DeltaTime 5.0)))

(fn CameraRotation
  (params (DeltaTime :type Float%20%28single-precision%29))
  (return (Math|Interpolation|RInterpTo (Transformation|GetActorRotation) (Variables|Default|GetDesiredRotation) DeltaTime 5.0)))