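; BP_LevelLoading is an actor that switches streamed sublevels on and off through two callable functions, with no active event logic of its own.
; LoadLevel prints the given level name, then sets that streaming level to load and become visible.
; ClearAllLevel unloads and hides the three hard-coded shape levels: triangle, hexagon and square.
; Both work by setting streaming-level flags directly rather than using latent load or unload nodes.
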(event EventBeginPlay)

(event Collision|EventActorBeginOverlap
  (params (OtherActor :type Actor%20Object%20Reference)))

(event EventTick
  (params (DeltaSeconds :type Float%20%28single-precision%29)))

(fn ConstructionScript)

(fn LoadLevel
  (params (LevelName :type String))
  (bind _returnvalue (Utilities|String|StringToName LevelName))
  (bind _returnvalue_2 (Class|GameplayStatics|GetStreamingLevel _returnvalue))
  (Development|PrintString LevelName)
  (Variables|/Script/Engine.LevelStreaming|SetbShouldBeLoaded _returnvalue_2 true)
  (Variables|/Script/Engine.LevelStreaming|SetbShouldBeVisible _returnvalue_2 true))

(fn ClearAllLevel
  (bind _returnvalue (Utilities|String|StringToName "L_Triangle"))
  (bind _returnvalue_2 (Utilities|String|StringToName "L_Square"))
  (bind _returnvalue_3 (Utilities|String|StringToName "L_Hexagone"))
  (bind _returnvalue_4 (Class|GameplayStatics|GetStreamingLevel _returnvalue_2))
  (bind _returnvalue_5 (Class|GameplayStatics|GetStreamingLevel _returnvalue))
  (bind _returnvalue_6 (Class|GameplayStatics|GetStreamingLevel _returnvalue_3))
  (Variables|/Script/Engine.LevelStreaming|SetbShouldBeLoaded _returnvalue_5 false)
  (Variables|/Script/Engine.LevelStreaming|SetbShouldBeVisible _returnvalue_5 false)
  (Variables|/Script/Engine.LevelStreaming|SetbShouldBeLoaded _returnvalue_6 false)
  (Variables|/Script/Engine.LevelStreaming|SetbShouldBeVisible _returnvalue_6 false)
  (Variables|/Script/Engine.LevelStreaming|SetbShouldBeLoaded _returnvalue_4 false)
  (Variables|/Script/Engine.LevelStreaming|SetbShouldBeVisible _returnvalue_4 false))