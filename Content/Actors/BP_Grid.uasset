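; BP_Grid is a grid actor that builds a flat tile grid of squares, hexagons or triangles as instanced static meshes.
; SpawnGrid takes mesh, size and material from DT_GridShapeData by shape name, then adds world-space instances around a center snapped to tile size.
; Helper functions derive each transform, staggering hexagon columns and flipping alternate triangles.
; The construction script's SpawnGrid call is disconnected, so nothing here triggers generation.
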(event EventBeginPlay)

(event Collision|EventActorBeginOverlap
  (params (OtherActor :type Actor%20Object%20Reference)))

(event EventTick
  (params (DeltaSeconds :type Float%20%28single-precision%29)))

(fn ConstructionScript)

(fn SpawnGrid
  (params (CenterLocation :type Vector) (TileSize :type Vector) (TileCount :type Vector%202D%20Structure) (Shape :type E_GridShape%20Enum :default "NewEnumerator0"))
  (bind _returnvalue (CallFunction|GetCurrentShapeData))
  (bind _instancedstaticmesh (Variables|Default|GetInstancedStaticMesh))
  (bind (_meshsize _mesh _materialinstance _flatmesh _flatbordermaterial) (Utilities|Struct|BreakGridShapeData _returnvalue))
  (Components|InstancedStaticMesh|ClearInstances (Variables|Default|GetInstancedStaticMesh))
  (Variables|GridParameters|SetGridCenterLocation CenterLocation)
  (Variables|GridParameters|SetGridTileScale TileSize)
  (Variables|GridParameters|SetGridTileCount (Class|KismetMathLibrary|ToRounded2D TileCount))
  ;[0.06771 0.04423 0.06664] Set Values of first Instance
  (Variables|GridParameters|SetShape Shape)
  (Components|StaticMesh|SetStaticMesh _instancedstaticmesh _flatmesh)
  (Variables|Default|SetMeshSize _meshsize)
  ;[0.06771 0.04423 0.06664] Create Instances
  (Rendering|Material|SetMaterial _instancedstaticmesh 0 _flatbordermaterial)
  (for _index (range 0 (- (Math|Float|Round (.x (Variables|GridParameters|GetGridTileCount))) 1))
    (Variables|Default|SetCurrentHorizontalIndex _index)
    (for _index_2 (range 0 (- (Math|Float|Round (.y (Variables|GridParameters|GetGridTileCount))) 1))
      ;[0.06771 0.04423 0.06664] Reset Center of Grid for snaping
      (Variables|Default|SetCurrentVerticalIndex _index_2)
      (Variables|GridParameters|SetGridCenterLocation (Utilities|Select :Index Shape :NewEnumerator0 "0, 0, 0" :NewEnumerator1 (CallFunction|SnapVectortoVector (Variables|GridParameters|GetGridCenterLocation) (* (Variables|GridParameters|GetGridTileScale) "1.000000,1.000000,0.000000")) :NewEnumerator2 (CallFunction|SnapVectortoVector (Variables|GridParameters|GetGridCenterLocation) (* (Variables|GridParameters|GetGridTileScale) "2.000000,1.000000,0.000000")) :NewEnumerator3 (CallFunction|SnapVectortoVector (Variables|GridParameters|GetGridCenterLocation) (* "2.000000,2.000000,0.000000" (Variables|GridParameters|GetGridTileScale)))))
      (Components|InstancedStaticMesh|AddInstance (Variables|Default|GetInstancedStaticMesh) (Math|Transform|MakeTransform (+ (CallFunction|CalculatePosition) "0.000000,0.000000,1.000000") (CallFunction|CalculateRotation) (CallFunction|CalculateScale)) true))))

(fn GetCurrentShapeData
  (bind _returnvalue (Utilities|GetDataTableRow "/Game/Art/Meshes/Grids/DT_GridShapeData.DT_GridShapeData" (Utilities|String|StringToName (Utilities|String|EnumtoString (Variables|GridParameters|GetShape))))
    (:then
      (return _returnvalue))))

(fn CalculateScale
  (return (/ (Variables|GridParameters|GetGridTileScale) (Variables|Default|GetMeshSize))))

(fn CalculatePosition
  (bind _returnvalue (CallFunction|CalculateBasePosition))
  (return (Utilities|Select :Index (Variables|GridParameters|GetShape) :NewEnumerator0 "0, 0, 0" :NewEnumerator1 (CallFunction|CalculateBasePosition) :NewEnumerator2 (+ (* (Math|Vector|SelectVector _returnvalue (+ _returnvalue (* (Variables|GridParameters|GetGridTileScale) "0.000000,0.500000,0.000000")) (CallFunction|FloatOdd (Math|Conversions|ToFloat(Integer) (Variables|Default|GetCurrentHorizontalIndex)))) "0.750000,1.000000,1.000000") (* (Variables|GridParameters|GetGridTileScale) "0.000000,0.500000,0.000000")) :NewEnumerator3 (* (CallFunction|CalculateBasePosition) "1.000000,0.500000,1.000000"))))

(fn CalculateRotation
  (return (Utilities|Select :Index (Variables|GridParameters|GetShape) :NewEnumerator0 "0, 0, 0" :NewEnumerator1 "0, 0, 0" :NewEnumerator2 "0, 0, 0" :NewEnumerator3 (Math|Rotator|MakeRotator 0.0 0.0 (+ 0.0 (Math|Float|SelectFloat 1.8e+02 0.0 (CallFunction|FloatOdd (Math|Conversions|ToFloat(Integer) (+ (Variables|Default|GetCurrentHorizontalIndex) (Variables|Default|GetCurrentVerticalIndex))))))))))

(fn CalculateBasePosition
  (bind _gridtilescale (Variables|GridParameters|GetGridTileScale))
  (return (- (Math|Conversions|ToVector(Vector2D) (* (- (- (Class|KismetMathLibrary|ToRounded2D (/ (Variables|GridParameters|GetGridTileCount) "(X=2.000000,Y=2.000000)")) "(X=1.000000,Y=1.000000)") (Math|Vector2D|MakeVector2D (Math|Conversions|ToFloat(Integer) (Variables|Default|GetCurrentHorizontalIndex)) (Math|Conversions|ToFloat(Integer) (Variables|Default|GetCurrentVerticalIndex)))) (Math|Vector2D|MakeVector2D (.x _gridtilescale) (.y _gridtilescale)))) (Variables|GridParameters|GetGridCenterLocation))))